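; BP_Plane is a static mesh actor that acts as a drop-off point for whatever the third-person character holds in its arm.
; When its mesh is hit by a ThirdPersonCharacter with InArm set, it increments that character's Level, clears InArm and empties the ArmMesh.
; It then prints the new Level, and all progression state lives on the character.
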(event `self.StaticMesh.OnComponentHit`
  (params (HitComponent :type "PrimitiveComponent Object Reference") (OtherActor :type "Actor Object Reference") (OtherComp :type "PrimitiveComponent Object Reference") (NormalImpulse :type "Vector Structure") (Hit :type "HitResult Structure (by ref)"))
  (bind _asthird_person_character (cast `/Game/ThirdPersonBP/Blueprints/ThirdPersonCharacter` OtherActor))
  (if (`/Game/ThirdPersonBP/Blueprints/ThirdPersonCharacter.inArm?` _asthird_person_character)
    (bind _output_get (set `/Game/ThirdPersonBP/Blueprints/ThirdPersonCharacter.level` (+ (`/Game/ThirdPersonBP/Blueprints/ThirdPersonCharacter.level` _asthird_person_character) 1) _asthird_person_character))
    (set `/Game/ThirdPersonBP/Blueprints/ThirdPersonCharacter.inArm?` false _asthird_person_character)
    (`StaticMeshComponent.SetStaticMesh` (`/Game/ThirdPersonBP/Blueprints/ThirdPersonCharacter.ArmMesh` _asthird_person_character) null)
    (`KismetSystemLibrary.PrintString` (`KismetStringLibrary.Conv_IntToString` _output_get))))

(fn `UserConstructionScript`)